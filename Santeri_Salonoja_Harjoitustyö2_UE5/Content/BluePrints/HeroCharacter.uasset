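; Player character for a twin-stick shooter that moves, aims, fires and dies.
; On BeginPlay it spawns a weapon onto the GunSocket, records its spawn transform in the game mode and creates the HUD.
; Move axes drive world-space movement, while look axes past a deadzone set control rotation and hold the weapon trigger.
; AffectHealth subtracts damage; at zero health it disables input, waits, requests a game mode respawn and destroys weapon and character.
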(event EventBeginPlay
  (bind _mesh (Variables|Character|GetMesh))
  (Utilities|FlowControl|Sequence
    (:then_0
      ;[0.15 0.15 0.15 0.5] Weapon spawn
      (bind _returnvalue (Game|SpawnActorfromClass "/Game/BluePrints/Weapon.Weapon_C" (Transformation|GetWorldTransform _mesh) "Undefined" "MultiplyWithRoot" 0 0))
      (bind _output_get (Variables|Default|SetWeapon _returnvalue))
      (Transformation|AttachComponentToComponent _output_get _mesh "GunSocket" "SnapToTarget" "SnapToTarget" "KeepWorld" true))
    (:then_1
      ;[0.15 0.15 0.15 0.5] Respawn transform
      (bind _astwin_shooter_game_mode (Utilities|Casting|CastToTwinShooterGameMode (Game|GetGameMode)))
      (bind _output_get_2 (Variables|Default|SetGame%20Mode _astwin_shooter_game_mode))
      (Variables|/Game/BluePrints/TwinShooterGameMode.TwinShooterGameMode_C|SetPlayerSpawnTransform _output_get_2 (Transformation|GetActorTransform)))
    (:then_2
      ;[0.15 0.15 0.15 0.5] HUD
      (bind _returnvalue_2 (UserInterface|CreateWidget "/Game/BluePrints/TwinStickHUD.TwinStickHUD_C"))
      (UserInterface|Viewport|AddtoViewport _returnvalue_2 0))))

(event Collision|EventActorBeginOverlap
  (params (OtherActor :type Actor%20Object%20Reference)))

(event EventTick
  (params (DeltaSeconds :type Float%20%28single-precision%29)))

(event EventAffectHealth
  (params (Delta :type Float%20%28double-precision%29))
  ;[0.15 0.15 0.15 0.5] Damage
  (Variables|Default|SetHealth (- (Variables|Default|GetHealth) Delta))
  (if (<= (Variables|Default|GetHealth) 0.0)
    ;[0.15 0.15 0.15 0.5] Death
    (Variables|Default|SetisDead true)
    (Input|DisableInput 0)
    (Utilities|FlowControl|Delay 3.0)
    (Default|RespawnPlayer (Variables|Default|GetGame%20Mode))
    (Actor|DestroyActor (Variables|Default|GetWeapon))))

(event Input|AxisEvents|InputAxisMoveUp
  (params (AxisValue :type Float%20%28single-precision%29))
  ;[0.15 0.15 0.15 0.5] Movement
  (Pawn|Input|AddMovementInput "1.000000,0.000000,0.000000" AxisValue false))

(event Input|AxisEvents|InputAxisMoveRight
  (params (AxisValue :type Float%20%28single-precision%29))
  ;[0.15 0.15 0.15 0.5] Movement
  (Pawn|Input|AddMovementInput "0.000000,1.000000,0.000000" AxisValue false))

(event Input|AxisEvents|InputAxisLookUp
  (params (AxisValue :type Float%20%28single-precision%29))
  (bind _weapon (Variables|Default|GetWeapon))
  ;[0.15 0.15 0.15 0.5] Rotation
  (if (> (Math|Vector|VectorLength (Math|Vector|MakeVector AxisValue (stale Input|AxisEvents|InputAxisLookRight AxisValue) 0.0)) 0.25)
    (Pawn|SetControlRotation (Pawn|GetController) (Math|Conversions|RotationFromXVector (Math|Vector|MakeVector AxisValue (stale Input|AxisEvents|InputAxisLookRight AxisValue) 0.0)))
    ;[0.15 0.15 0.15 0.5] Weapon fire
    (Default|PullTrigger _weapon)
    (else
      (Default|ReleaseTrigger _weapon))))

(event Input|AxisEvents|InputAxisLookRight
  (params (AxisValue :type Float%20%28single-precision%29))
  (bind _weapon (Variables|Default|GetWeapon))
  ;[0.15 0.15 0.15 0.5] Rotation
  (if (> (Math|Vector|VectorLength (Math|Vector|MakeVector (stale Input|AxisEvents|InputAxisLookUp AxisValue) AxisValue 0.0)) 0.25)
    (Pawn|SetControlRotation (Pawn|GetController) (Math|Conversions|RotationFromXVector (Math|Vector|MakeVector (stale Input|AxisEvents|InputAxisLookUp AxisValue) AxisValue 0.0)))
    ;[0.15 0.15 0.15 0.5] Weapon fire
    (Default|PullTrigger _weapon)
    (else
      (Default|ReleaseTrigger _weapon))))

(fn ConstructionScript)